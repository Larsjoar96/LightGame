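; DeathZone_BP is a death zone actor meant to show the lose screen when the player overlaps it.
; BeginPlay caches the player character as MyPlayer_BP.
; On overlap, it compares the other actor to the cached player's RootComponent, not to the player actor itself.
; A match creates the LoseMenu widget, adds it to the viewport and switches input to UI only.
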(event EventBeginPlay
  (bind _asmy_player_bp (Utilities|Casting|CastToMyPlayer_BP (Game|GetPlayerCharacter 0)))
  (Variables|Default|SetPlayer _asmy_player_bp))

(event Collision|EventActorBeginOverlap
  (params (OtherActor :type Actor%20Object%20Reference))
  (bind _returnvalue (Game|GetPlayerController 0))
  (if (== OtherActor (Variables|/Script/Engine.Actor|GetRootComponent (Variables|Default|GetPlayer)))
    (bind _returnvalue_2 (UserInterface|CreateWidget "/Game/HUD/LoseMenu.LoseMenu_C" _returnvalue))
    (UserInterface|Viewport|AddtoViewport _returnvalue_2 0)
    (Input|SetInputModeUIOnly _returnvalue _returnvalue_2 "DoNotLock")))

(event EventTick
  (params (DeltaSeconds :type Float%20%28single-precision%29)))

(fn ConstructionScript)