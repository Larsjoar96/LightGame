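; Spawner actor that spawns a single Enemy_BP when the player comes within its trigger sphere.
; BeginPlay caches the MyPlayer_BP character, and Sphere1's overlap event fires the spawn only for that player's capsule component.
; The enemy appears at the spawner's transform with navigation-generation influence disabled, then the spawner destroys itself, making it one-shot.
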(event OnComponentBeginOverlap(Sphere1)
  (params (OverlappedComponent :type Primitive%20Component%20Object%20Reference) (OtherActor :type Actor%20Object%20Reference) (OtherComp :type Primitive%20Component%20Object%20Reference) (OtherBodyIndex :type Integer) (bFromSweep :type Boolean) (SweepResult :type Hit%20Result%20Structure%20%28by%20ref%29))
  (if (== OtherComp (Variables|/Script/Engine.Character|GetCapsuleComponent (Variables|Default|GetPlayerRef)))
    (CallFunction|SpawnEnemy)))

(event Custom|Spawn%20Enemy
  (bind _returnvalue (Game|SpawnActorfromClass "/Game/AI/Enemy_BP.Enemy_BP_C" (Transformation|GetActorTransform) "Undefined" 0 0))
  (Class|Pawn|SetCanAffectNavigationGeneration _returnvalue false)
  (Actor|DestroyActor))

(event Collision|EventActorBeginOverlap
  (params (OtherActor :type Actor%20Object%20Reference)))

(event EventTick
  (params (DeltaSeconds :type Float%20%28single-precision%29)))

(event EventBeginPlay
  (bind _asmy_player_bp (Utilities|Casting|CastToMyPlayer_BP (Game|GetPlayerCharacter 0)))
  (Variables|Default|SetPlayerRef _asmy_player_bp))

(fn ConstructionScript)