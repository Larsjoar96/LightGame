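; Enemy character that damages the player on contact and can be slowed, then stunned, by the player's flashlight cone.
; Overlap with the cone drives a per-frame exposure counter, reducing walk speed and swapping materials until the stun threshold freezes it.
; Die destroys it only while weakened.
; Leaving the cone clears weakness and drains the counter, with speed and default material restored only at zero.
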(event OnComponentBeginOverlap(AttackCollider)
  (params (OverlappedComponent :type Primitive%20Component%20Object%20Reference) (OtherActor :type Actor%20Object%20Reference) (OtherComp :type Primitive%20Component%20Object%20Reference) (OtherBodyIndex :type Integer) (bFromSweep :type Boolean) (SweepResult :type Hit%20Result%20Structure%20%28by%20ref%29))
  ;[1 1 1] Deal Damage
  (if (== OtherComp (Variables|/Script/Engine.Character|GetCapsuleComponent (Variables|Default|GetPlayerRef)))
    (Default|TakeDamage (Variables|Default|GetPlayerRef))))

(event OnComponentBeginOverlap(Box)
  (params (OverlappedComponent :type Primitive%20Component%20Object%20Reference) (OtherActor :type Actor%20Object%20Reference) (OtherComp :type Primitive%20Component%20Object%20Reference) (OtherBodyIndex :type Integer) (bFromSweep :type Boolean) (SweepResult :type Hit%20Result%20Structure%20%28by%20ref%29))
  (if (== OtherComp (Variables|/Game/Blueprints/TopDownCharacter_BP.TopDownCharacter_BP_C|GetCone (Variables|Default|GetPlayerRef)))
    (Variables|Default|SetBeingWeakened true)))

(event OnComponentEndOverlap(Box)
  (params (OverlappedComponent :type Primitive%20Component%20Object%20Reference) (OtherActor :type Actor%20Object%20Reference) (OtherComp :type Primitive%20Component%20Object%20Reference) (OtherBodyIndex :type Integer))
  (if (== OtherComp (Variables|/Game/Blueprints/TopDownCharacter_BP.TopDownCharacter_BP_C|GetCone (Variables|Default|GetPlayerRef)))
    (Variables|Default|SetBeingWeakened false)
    (Variables|Default|SetIsWeak false)))

(event Custom|Weakening
  ;[1 1 1] Weakening Enemies
  (if (>= (Variables|Default|GetFlashLightTime) (Variables|Default|GetStunTime))
    (Variables|Default|SetIsWeak true)
    (Variables|/Script/Engine.CharacterMovementComponent|SetMaxWalkSpeed (Variables|Character|GetCharacterMovement) 0.0)
    (Rendering|Material|SetMaterial (Variables|Character|GetMesh) 0 "/Game/Materials/MEnemyWeakened.MEnemyWeakened")
    (else
      (Variables|Default|SetIsWeak false)
      (Variables|/Script/Engine.CharacterMovementComponent|SetMaxWalkSpeed (Variables|Character|GetCharacterMovement) (- (Variables|Default|GetTopSpeed) (Variables|Default|GetFlashLightTime)))
      (Rendering|Material|SetMaterial (Variables|Character|GetMesh) 0 "/Game/Materials/MEnemyWeakening.MEnemyWeakening"))))

(event Custom|Die
  (if (Variables|Default|GetIsWeak)
    (Actor|DestroyActor)))

(event Custom|Rally
  (Variables|Default|SetIsWeak false)
  (Variables|Default|SetBeingWeakened false)
  (Variables|/Script/Engine.CharacterMovementComponent|SetMaxWalkSpeed (Variables|Character|GetCharacterMovement) 3e+02)
  (Rendering|Material|SetMaterial (Variables|Character|GetMesh) 0 "/Game/Materials/MEnemyDefault.MEnemyDefault"))

(event EventBeginPlay
  ;[1 1 1] Set Player Reference
  (bind _astop_down_character_bp (Utilities|Casting|CastToTopDownCharacter_BP (Game|GetPlayerCharacter 0)))
  (Variables|Default|SetPlayerRef _astop_down_character_bp))

(event EventTick
  (params (DeltaSeconds :type Float%20%28single-precision%29))
  ;[1 1 1] Weakening Enemies
  (if (Variables|Default|GetBeingWeakened)
    (if (< (Variables|Default|GetFlashLightTime) 1.8e+02)
      (Variables|Default|SetFlashLightTime (+ (Variables|Default|GetFlashLightTime) 1.0))
      (CallFunction|Weakening)
      (else
        (CallFunction|Weakening)))
    (else
      (Variables|Default|SetFlashLightTime (- (Variables|Default|GetFlashLightTime) 1.0))
      (if (<= (Variables|Default|GetFlashLightTime) 0.0)
        (Variables|Default|SetFlashLightTime 0.0)
        (CallFunction|Rally)
        (else
          (Rendering|Material|SetMaterial (Variables|Character|GetMesh) 0 "/Game/Materials/MEnemyWeakening.MEnemyWeakening"))))))

(fn ConstructionScript)